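; BP_ArenaCharacter is the playable arena character, moved on diagonal world axes and turned by swing inputs that set control rotation past a dead zone.
; On BeginPlay it caches the game mode, fills health and uses physical animation to simulate physics on both arms and the spine down.
; Damage reduces clamped health, and death calls PlayerDead before destroying the actor.
; Per-player colouring is unwired, and cube overlap only casts.
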(event `InputAxis|SwingLeft`
  (params (AxisValue :type "Float (single-precision)"))
  ;[1 1 1] Swing Left and Right
  (bind _returnvalue (`KismetMathLibrary.MakeVector` AxisValue (stale `InputAxis|SwingRight` AxisValue)))
  (if (> (`KismetMathLibrary.VSize` _returnvalue) 0.25) :!label _label
    (`Controller.SetControlRotation` (`self.GetController`) (`KismetMathLibrary.Conv_VectorToRotator` _returnvalue))))

(event `InputAxis|MoveVertical`
  (params (AxisValue :type "Float (single-precision)"))
  ;[1 1 1] Movement
  (`self.AddMovementInput` (1.0 -1.0 0.0) AxisValue))

(event `InputAxis|SwingRight`
  (params (AxisValue :type "Float (single-precision)"))
  ;[1 1 1] Swing Left and Right
  (goto _label))

(event `InputAxis|MoveHorizontal`
  (params (AxisValue :type "Float (single-precision)"))
  ;[1 1 1] Movement
  (`self.AddMovementInput` (1.0 1.0 0.0) AxisValue))

(event `self.ReceiveBeginPlay`
  ;[1 1 1] Sets Game Mode Ref
  (bind _asbp_arena_game_mode (cast `/Game/DeadArms/Core/BP_ArenaGameMode` (`GameplayStatics.GetGameMode`)))
  (set `self.GameModeRef` _asbp_arena_game_mode)
  ;[1 0 0] Sets Physics Anims
  (`self.PhysicsAnimations`)
  (`self.PlayerStats`))

(event `self.ReceiveAnyDamage`
  (params (Damage :type "Float (single-precision)") (DamageType :type "DamageType Object Reference") (InstigatedBy :type "Controller Object Reference") (DamageCauser :type "Actor Object Reference"))
  (set `self.IncomingDamage` Damage)
  (set `self.CurrentHealth` (`KismetMathLibrary.FClamp` (- (`self.CurrentHealth`) (`self.IncomingDamage`)) 0.0 (`self.MaxHealth`)))
  (if (<= (`self.CurrentHealth`) 0.0)
    (`self.PlayerDeath`)))

(event `PlayerDeath`
  (`self.PlayerDead`)
  (`self.K2_DestroyActor`)
  (`KismetSystemLibrary.PrintString` "Hello"))

(event `self.ReceiveTick`
  (params (DeltaSeconds :type "Float (single-precision)")))

(event `self.Cube.OnComponentBeginOverlap`
  (params (OverlappedComponent :type "PrimitiveComponent Object Reference") (OtherActor :type "Actor Object Reference") (OtherComp :type "PrimitiveComponent Object Reference") (OtherBodyIndex :type Integer) (bFromSweep :type Boolean) (SweepResult :type "HitResult Structure (by ref)"))
  (cast `/Game/DeadArms/Core/Character/BP_ArenaCharacter` OtherActor))

(fn `PhysicsAnimations`
  (bind _physicalanimation (`self.PhysicalAnimation`))
  (bind _mesh (`self.Mesh`))
  (bind _physicsprofilename (`self.PhysicsProfileName`))
  (bind _leftarmbonename (`self.LeftArmBoneName`))
  (bind _spinebonename (`self.SpineBoneName`))
  (bind _rightarmbonename (`self.RightArmBoneName`))
  (`PhysicalAnimationComponent.SetSkeletalMeshComponent` (`self.PhysicalAnimation`) (`self.Mesh`))
  (`|ExecutionSequence`
    (:`then_0`
      ;[1 1 1] Left Arm Simulate Physics
      (`PhysicalAnimationComponent.ApplyPhysicalAnimationProfileBelow` _physicalanimation _leftarmbonename _physicsprofilename true false)
      (`SkeletalMeshComponent.SetAllBodiesBelowSimulatePhysics` _mesh _leftarmbonename true true))
    (:`then_1`
      ;[1 1 1] Right Arm Simulate Physics
      (`PhysicalAnimationComponent.ApplyPhysicalAnimationProfileBelow` _physicalanimation _rightarmbonename _physicsprofilename true false)
      (`SkeletalMeshComponent.SetAllBodiesBelowSimulatePhysics` _mesh _rightarmbonename true true))
    (:`then_2`
      ;[1 1 1] Upper Body Simulate Physics
      (`PhysicalAnimationComponent.ApplyPhysicalAnimationProfileBelow` _physicalanimation _spinebonename _physicsprofilename true false)
      (`SkeletalMeshComponent.SetAllBodiesBelowSimulatePhysics` _mesh _spinebonename true true))))

(fn `PlayerStats`
  (set `self.CurrentHealth` (`self.MaxHealth`)))

(fn `UserConstructionScript`)