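; BP_ArenaFighter is an arena fighter character that tints its body to show which player controls it.
; A DoOnce on Tick, rather than BeginPlay, casts the controller to BP_ArenaPlayerController and reads its player controller ID.
; It creates a dynamic instance of the mannequin body material and sets BodyColor to a distinct colour for each of four player IDs.
; BeginPlay and the construction script only call their parents.
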(event `self.ReceiveBeginPlay`
  (`parent.ReceiveBeginPlay`))

(event `self.ReceiveTick`
  (params (DeltaSeconds :type "Float (single-precision)"))
  ;[1 1 1] Kinda bad Code but it only works if i do it this way.. RIP / Gets player controller ID and sets a colour for them
  (`parent.ReceiveTick` DeltaSeconds)
  (`/Engine/EditorBlueprintResources/StandardMacros.DoOnce` false
    (:`Completed`
      (bind _asbp_arena_player_controller (cast `/Game/DeadArms/Core/BP_ArenaPlayerController` (`self.GetController`)))
      (bind _returnvalue (`GameplayStatics.GetPlayerControllerID` _asbp_arena_player_controller))
      (bind _returnvalue_2 (`PrimitiveComponent.CreateDynamicMaterialInstance` (`self.Mesh`) 0 "/Game/Mannequin/Character/Materials/M_UE4Man_Body_Inst.M_UE4Man_Body_Inst"))
      (switch `int` _returnvalue
        (:`0`
          (`MaterialInstanceDynamic.SetVectorParameterValue` _returnvalue_2 "BodyColor" (struct :`R` 0.769097 :`G` 0.077027 :`B` 0.099983 :`A` 1.0)))
        (:`1`
          (`MaterialInstanceDynamic.SetVectorParameterValue` _returnvalue_2 "BodyColor" (struct :`R` 0.20241 :`G` 0.177122 :`B` 0.633681 :`A` 1.0)))
        (:`2`
          (`MaterialInstanceDynamic.SetVectorParameterValue` _returnvalue_2 "BodyColor" (struct :`R` 0.293285 :`G` 0.866319 :`B` 0.353091 :`A` 1.0)))
        (:`3`
          (`MaterialInstanceDynamic.SetVectorParameterValue` _returnvalue_2 "BodyColor" (struct :`R` 0.998475 :`G` 0.351401 :`B` 1.0 :`A` 1.0)))))))

(fn `UserConstructionScript`
  (`parent.UserConstructionScript`))