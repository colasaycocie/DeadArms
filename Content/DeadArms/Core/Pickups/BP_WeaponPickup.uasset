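; BP_WeaponPickup is a weapon pickup actor that prints a message and destroys itself on its PickUp event.
; BeginPlay looks up the Baseballbat row in WeaponTable but does nothing with the result.
; A disconnected Hammer lookup would set Damage and both hand weapon meshes, but it never runs, so pickup grants no weapon here.
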(event `self.ReceiveBeginPlay`
  (bind _returnvalue (`|GetDataTableRow` "/Game/DeadArms/Core/Pickups/WeaponTable.WeaponTable" "Baseballbat")))

(event `/Game/DeadArms/Core/BP_WeaponInterface.PickUp`
  (`KismetSystemLibrary.PrintString` "You Have Picked Up the Item!")
  (`self.K2_DestroyActor`))

(fn `UserConstructionScript`)