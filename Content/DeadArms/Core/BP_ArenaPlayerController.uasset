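; BP_ArenaPlayerController is the player controller for the arena, letting the player spawn and despawn their character by key press.
; On BeginPlay it casts the game mode to BP_ArenaGameMode and caches it.
; Space calls SpawnCharacter and Backspace calls DespawnPlayer on that game mode, passing itself and printing a debug string.
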(event `self.ReceiveBeginPlay`
  (bind _asbp_arena_game_mode (cast `/Game/DeadArms/Core/BP_ArenaGameMode` (`GameplayStatics.GetGameMode`)))
  (set `self.ArenaGameMode` _asbp_arena_game_mode))

(event `Key|SpaceBar`
  (params (Key :type "Key Structure"))
  (:`Pressed`
    (`/Game/DeadArms/Core/BP_ArenaGameMode.SpawnCharacter` (`self.ArenaGameMode`) self)
    (`KismetSystemLibrary.PrintString` "Spawn Character")))

(event `Key|BackSpace`
  (params (Key :type "Key Structure"))
  (:`Pressed`
    (`/Game/DeadArms/Core/BP_ArenaGameMode.DespawnPlayer` (`self.ArenaGameMode`) self)
    (`KismetSystemLibrary.PrintString` "DeSpawn Character")))

(fn `UserConstructionScript`)