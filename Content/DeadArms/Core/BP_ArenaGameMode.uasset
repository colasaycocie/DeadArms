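; Arena game mode that creates four local players at start and handles fighter respawn and despawn.
; BeginPlay caches the level's PlayerStarts before creating the players.
; SpawnCharacter replaces a controller's pawn with a possessed BP_ArenaFighter and records it in Players, while DespawnPlayer swaps an existing pawn for a SpectatorPawn.
; Both take transforms from GetRandomSpawn, whose random PlayerStart lookup appears unconnected.
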(event `self.ReceiveBeginPlay`
  (bind _outactors (`GameplayStatics.GetAllActorsOfClass` "/Script/Engine.PlayerStart"))
  (set `self.PlayerStartArray` _outactors)
  ;[1 1 1] Sets Max Players to 4
  (for _index (range 4)
    (`GameplayStatics.CreatePlayer` _index)))

(event `SpawnCharacter`
  (params (`Player Controller` :type "Controller Object Reference"))
  (bind _returnvalue (`Controller.K2_GetPawn` `Player Controller`))
  ;[1 1 1] Respawn
  (`/Engine/EditorBlueprintResources/StandardMacros.IsValid` _returnvalue
    (:`Is Valid`
      (`self.K2_DestroyActor` _returnvalue))
    (:`Is Not Valid`
      _))
  (bind _returnvalue_2 (`|SpawnActorFromClass` "/Game/DeadArms/Core/Character/BP_ArenaFighter.BP_ArenaFighter_C" (`self.GetRandomSpawn`) "AdjustIfPossibleButAlwaysSpawn" "OverrideRootScale" null null))
  (`Controller.Possess` `Player Controller` _returnvalue_2)
  (`KismetArrayLibrary.Array_AddUnique` (`self.Players`) _returnvalue_2))

(event `DespawnPlayer`
  (params (`Player Controller` :type "Controller Object Reference"))
  (bind _returnvalue (`Controller.K2_GetPawn` `Player Controller`))
  (`/Engine/EditorBlueprintResources/StandardMacros.IsValid` _returnvalue
    (:`Is Valid`
      (`self.K2_DestroyActor` _returnvalue)
      (bind _returnvalue_2 (`|SpawnActorFromClass` "/Script/Engine.SpectatorPawn" (`self.GetRandomSpawn`) "AdjustIfPossibleButAlwaysSpawn" "OverrideRootScale" null null))
      (`Controller.Possess` `Player Controller` _returnvalue_2))))

(fn `UserConstructionScript`)