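; BP_Camera is a shared arena camera that zooms according to how far apart the players are.
; Every tick, ClassSetup reads the Players list from BP_ArenaGameMode and makes this camera the view target of all player controllers.
; It then sets the spring arm length to the largest pairwise distance among four players, addressed by fixed indices, with no clamping or smoothing.
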(event `self.ReceiveTick`
  (params (DeltaSeconds :type "Float (single-precision)"))
  (`self.Class Setup`))

(fn `Class Setup`
  (bind _asbp_arena_game_mode (cast `/Game/DeadArms/Core/BP_ArenaGameMode` (`GameplayStatics.GetGameMode`)))
  (bind _output_get (set `self.BP_GameMode` _asbp_arena_game_mode))
  (bind _output_get_2 (set `self.PlayersReference` (`/Game/DeadArms/Core/BP_ArenaGameMode.Players` _output_get)))
  (bind _outactors (`GameplayStatics.GetAllActorsOfClass` "/Script/Engine.PlayerController"))
  (`PlayerController.SetViewTargetWithBlend` _outactors self 0.0 "VTBlend_Linear" 0.0 false)
  (bind _output (`|GetArrayItem` _output_get_2))
  (bind _output_2 (`|GetArrayItem` _output_get_2 1))
  (bind _output_3 (`|GetArrayItem` _output_get_2 2))
  (bind _output_4 (`|GetArrayItem` _output_get_2 3))
  (set `SpringArmComponent.TargetArmLength` (`.MaxValue` (`KismetMathLibrary.MaxOfFloatArray` (`|MakeArray` (`self.GetDistanceTo` _output _output_2) (`self.GetDistanceTo` _output _output_3) (`self.GetDistanceTo` _output_2 _output_3) (`self.GetDistanceTo` _output _output_4) (`self.GetDistanceTo` _output_2 _output_4) (`self.GetDistanceTo` _output_3 _output_4)))) (`self.SpringArm`)))

(fn `UserConstructionScript`)