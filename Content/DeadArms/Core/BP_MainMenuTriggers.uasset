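; BP_MainMenuTriggers is an overlap-driven main menu trigger that either opens the Arena_P level or quits the game, depending on its LoadLevel setting.
; Beginning an overlap clears the BreakSequence flag and starts a two-second delay before the chosen action runs.
; Ending the overlap sets the flag, which cancels the action unless a new overlap clears it before the delay completes.
; Overlapping actors are not filtered.
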(event `self.ReceiveActorBeginOverlap`
  (params (OtherActor :type "Actor Object Reference"))
  ;[1 1 1] On Overlap an action is triggered, load level or quit game
  (set `self.BreakSequence?` false)
  (switch `/Game/DeadArms/Core/EMainMenuOption` "NewEnumerator0"
    (:`NewEnumerator0`
      (`KismetSystemLibrary.Delay` 2.0)
      (if (not (`self.BreakSequence?`))
        (`GameplayStatics.OpenLevel` "Arena_P")))
    (:`NewEnumerator1`
      (`KismetSystemLibrary.Delay` 2.0)
      (if (not (`self.BreakSequence?`))
        (`KismetSystemLibrary.QuitGame` null "Quit")))))

(event `self.ReceiveActorEndOverlap`
  (params (OtherActor :type "Actor Object Reference"))
  ;[1 1 1] If the actor stops overlapping, break the sequence
  (set `self.BreakSequence?` true))

(fn `UserConstructionScript`)