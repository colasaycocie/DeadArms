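; Shared arena camera that follows all BP_ArenaFighter actors and becomes player 0's view target every tick.
; Each tick it gathers fighter X/Y positions and moves its root to their bounding-box midpoint at fixed height.
; Spring arm length is the clamped length of the max-X/max-Y vector, measured from world origin rather than fighter spread.
; An older two-player, distance-based zoom remains in ClassSetup as unexecuted nodes.
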(event `self.ReceiveTick`
  (params (DeltaSeconds :type "Float (single-precision)"))
  (bind _xvalues (`self.XValues`))
  (bind _yvalues (`self.YValues`))
  (bind _xvalues_2 (`self.XValues`))
  (bind _yvalues_2 (`self.YValues`))
  (bind _returnvalue (`KismetMathLibrary.MakeVector` (`.MaxValue` (`KismetMathLibrary.MaxOfFloatArray` _xvalues)) (`.MaxValue` (`KismetMathLibrary.MaxOfFloatArray` _yvalues))))
  (bind _outactors (`GameplayStatics.GetAllActorsOfClass` "/Game/DeadArms/Core/Character/BP_ArenaFighter.BP_ArenaFighter_C"))
  (bind _output_get (set `self.Players` _outactors))
  (`PlayerController.SetViewTargetWithBlend` (`GameplayStatics.GetPlayerController` 0) self 0.0 "VTBlend_Linear" 0.0 false)
  (for _array_element _output_get
    (bind (_returnvalue_x _returnvalue_y) (`KismetMathLibrary.BreakVector` (`self.K2_GetActorLocation` _array_element)))
    (`KismetArrayLibrary.Array_AddUnique` _xvalues_2 _returnvalue_x)
    (`KismetArrayLibrary.Array_AddUnique` _yvalues_2 _returnvalue_y))
  (`SceneComponent.K2_SetWorldLocation` (`self.DefaultSceneRoot`) (`KismetMathLibrary.MakeVector` (.x (- _returnvalue (/ (- _returnvalue (`KismetMathLibrary.MakeVector` (`.MinValue` (`KismetMathLibrary.MinOfFloatArray` _xvalues)) (`.MinValue` (`KismetMathLibrary.MinOfFloatArray` _yvalues)))) 2))) (.y (- _returnvalue (/ (- _returnvalue (`KismetMathLibrary.MakeVector` (`.MinValue` (`KismetMathLibrary.MinOfFloatArray` _xvalues)) (`.MinValue` (`KismetMathLibrary.MinOfFloatArray` _yvalues)))) 2))) 800.0) true false)
  (set `SpringArmComponent.TargetArmLength` (`KismetMathLibrary.FClamp` (`KismetMathLibrary.VSize` _returnvalue) 0.0 500.0) (`self.SpringArm`))
  (`KismetArrayLibrary.Array_Clear` _yvalues_2)
  (`KismetArrayLibrary.Array_Clear` _xvalues_2))

(fn `Class Setup`
  (bind _outactors (`GameplayStatics.GetAllActorsOfClass` "/Game/DeadArms/Core/BP_ArenaPlayerController.BP_ArenaPlayerController_C")))

(fn `UserConstructionScript`)